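; Tracker is a selectable actor that plays a curve-driven motion around its own location and represents a particular WhichCharacter.
; On BeginPlay it initializes curves, injects them into the Movement timeline's tracks, then plays it to orient Center, scale PointOnSphere and roll RotatingStuff.
; Selection turns the cube light blue and broadcasts WhichCharacter; GetUnselected restores dark blue when another character is selected.
; TimelineFinished is an empty event.
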(event Custom|GetSelected
  (Rendering|Material|SetMaterial (Variables|Default|GetStaticCube) 0 "/Game/Assets/Materials/MI_LightBlue.MI_LightBlue"))

(event Custom|GetUnselected
  (params (WhoGotSelected :type E_WhichCharacter%20Enum :default "NewEnumerator0"))
  (if (not (Utilities|Enum|Equal(Enum) WhoGotSelected (Variables|Tracker|GetWhichCharacter)))
    (Rendering|Material|SetMaterial (Variables|Default|GetStaticCube) 0 "/Game/Assets/Materials/MI_DarkBlue.MI_DarkBlue")))

(event Custom|InitTimeline
  (bind _movement (Variables|Default|GetMovement))
  (Class|TimelineComponent|SetFloatCurve _movement (Variables|Default|GetXDeg_0) "XDeg")
  (Class|TimelineComponent|SetFloatCurve _movement (Variables|Default|GetYDeg_0) "YDeg")
  (Class|TimelineComponent|SetFloatCurve _movement (Variables|Default|GetZDeg_0) "Zdeg")
  (Class|TimelineComponent|SetFloatCurve _movement (Variables|Default|GetScale_0) "Scale")
  (CallFunction|StartTimeline))

(event Custom|StartTimeline
  (bind (_direction _xdeg _ydeg _zdeg _scale) (Timeline|Movement PlayFromStart)
    (:Update
      (Transformation|SetWorldTransform (Variables|Default|GetCenter) (Math|Transform|MakeTransform (Transformation|GetActorLocation) (Math|Rotator|MakeRotator 0.0 _ydeg _zdeg) "1,1,1") false false)
      (Transformation|SetRelativeScale3D (Variables|Default|GetPointOnSphere) (Math|Conversions|ToVector(Float) _scale))
      (Transformation|SetRelativeRotation (Variables|Default|GetRotatingStuff) (Math|Rotator|MakeRotator _xdeg 0.0 0.0) false false))
    (:Finished
      (CallFunction|TimelineFinished))))

(event Custom|TimelineFinished)

(event EventBeginPlay
  (Class|TrackerBase|InitalizeCurves)
  (CallFunction|InitTimeline))

(event EventOnSelect
  (CallFunction|GetSelected)
  (Default|CallGotSelected (Variables|Tracker|GetWhichCharacter)))

(fn ConstructionScript)