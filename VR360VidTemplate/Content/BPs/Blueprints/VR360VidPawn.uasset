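; Pawn for viewing 360 video that opens a 1080p demo media source at BeginPlay.
; Holding right mouse turns the actor, with optional inverted input and clamped pitch.
; Left click traces from the Hand component to a point ahead of the camera and sends OnSelectMessage to the hit actor.
; A second camera object trace also runs but its result is unused, and debug drawing and miss printing remain.
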(event EventBeginPlay
  (Default|Open (Variables|Default|GetMediaManager) "/Game/Movies/Demo1080pSource.Demo1080pSource"))

(event Input|MouseEvents|MouseX
  (params (AxisValue :type Float%20%28single-precision%29))
  (bind _returnvalue (Transformation|GetActorRotation))
  (if (Variables|Default|GetbIsRightMousePressed)
    (Transformation|SetActorRotation (Math|Rotator|MakeRotator 0.0 (.pitch _returnvalue) (+ (select (Variables|Default|GetbInvertMouseControls) (* -1 AxisValue) AxisValue) (.yaw _returnvalue))))))

(event Input|MouseEvents|MouseY
  (params (AxisValue :type Float%20%28single-precision%29))
  (bind _returnvalue (Transformation|GetActorRotation))
  (if (Variables|Default|GetbIsRightMousePressed)
    (Transformation|SetActorRotation (Math|Rotator|MakeRotator 0.0 (Math|Float|Clamp(Float) (+ (.pitch _returnvalue) (select (Variables|Default|GetbInvertMouseControls) (* -1 AxisValue) AxisValue)) -85.0 85.0) (.yaw _returnvalue)))))

(event Input|MouseEvents|RightMouseButton
  (params (Key :type Key%20Structure :default "None"))
  (:Pressed
    (Variables|Default|SetbIsRightMousePressed true))
  (:Released
    (Variables|Default|SetbIsRightMousePressed false)))

(event Input|MouseEvents|LeftMouseButton
  (params (Key :type Key%20Structure :default "None"))
  (bind _camera (Variables|Default|GetCamera))
  (bind _returnvalue (Transformation|GetWorldLocation _camera))
  (bind _returnvalue_2 (Math|Vector|GetForwardVector _camera))
  (bind _returnvalue_3 (* _returnvalue_2 1000))
  (bind _returnvalue_4 (+ _returnvalue _returnvalue_3))
  (:Pressed
    (bind _outhit (Collision|LineTraceForObjects _returnvalue _returnvalue_4 (Utilities|Array|MakeArray "ObjectTypeQuery1") false (Utilities|Array|MakeArray self) "None"))
    (bind (_outhit_2 _returnvalue_5) (Collision|LineTraceByChannel (Transformation|GetWorldLocation (Variables|Default|GetHand)) _returnvalue_4 "TraceTypeQuery3" false 0 "ForDuration" true "(R=1.000000,G=0.000000,B=0.000000,A=1.000000)" "(R=0.000000,G=1.000000,B=0.000000,A=1.000000)" 0.5))
    (if _returnvalue_5
      (Class|SelectInterface|OnSelect(Message) (.HitActor (Collision|BreakHitResult _outhit_2)))
      (else
        (Development|PrintString "you  missed")))))

(fn ConstructionScript)