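; LightBP is a light actor that flickers by animating an emissive parameter on its sphere's dynamic material.
; StartFlicker waits a short random delay, then Flicker reschedules itself on a randomized timer until StopFlicker clears it.
; Each tick a FlipFlop alternates between random dim and bright targets, passed to RampEmissive.
; RampEmissive lerps from the current value via a timeline whose play rate is scaled by RampDuration.
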(event Custom|StartFlicker
  (Utilities|FlowControl|Delay (Math|Random|RandomFloatinRange 0.0 0.5))
  (CallFunction|Flicker))

(event Custom|Flicker
  (Utilities|FlowControl|FlipFlop
    (:A
      (CallFunction|RampEmissive (Math|Random|RandomFloatinRange 1e+01 2e+01)))
    (:B
      (CallFunction|RampEmissive (Math|Random|RandomFloatinRange 3e+01 5e+01))))
  (bind _returnvalue (Utilities|Time|SetTimerbyEvent (delegate Custom|Flicker) (Math|Random|RandomFloatinRange 0.4 0.6)))
  (Variables|Default|SetHandle _returnvalue))

(event Custom|StopFlicker
  (Utilities|Time|ClearandInvalidateTimerbyHandle (Variables|Default|GetHandle)))

(event Custom|RampEmissive
  (params (End :type Float%20%28single-precision%29))
  (Components|Timeline|SetPlayRate (Variables|Default|GetTimeline_0) (/ 1.0 (Variables|Default|GetRampDuration)))
  (bind _newtrack_0 (Timeline|Timeline_0 PlayFromStart)
    (:Update
      (Rendering|Material|SetScalarParameterValue (Variables|Default|GetDynamicMat) (Variables|Default|GetEmissiveName) (Math|Float|Lerp (Variables|Default|GetCurrentEmissive) End _newtrack_0) :!class /Script/Engine.MaterialInstanceDynamic))
    (:Finished
      (Variables|Default|SetCurrentEmissive End))))

(event EventBeginPlay
  (bind _sphere (Variables|Default|GetSphere))
  (bind _returnvalue (Rendering|Material|CreateDynamicMaterialInstance _sphere 0 (Rendering|Material|GetMaterial _sphere 0) "None" :!class /Script/Engine.PrimitiveComponent))
  (Variables|Default|SetDynamicMat _returnvalue))

(fn ConstructionScript)